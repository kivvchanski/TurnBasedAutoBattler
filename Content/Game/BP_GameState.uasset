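; Game state that runs a turn-based 1v1 fighter game, from player setup to a win screen at five defeated enemies.
; BeginPlay and ResetGame spawn the player and TurnSystemManager if needed, then open the first-upgrade widget.
; InitPlayer applies the chosen DT_Classes row and random stats; it and NextFight spawn mobs at tagged TargetPoints.
; NewFight1v1 orders turns by comparing one stat; OnEnemyDown counts kills and clears finished fights.
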(event `ResetGame`
  (set `self.CountOfBeatedEnemies` 0)
  (bind _outactors (`GameplayStatics.GetAllActorsOfClass` "/Game/Game/BP_Fighter.BP_Fighter_C"))
  (for _array_element _outactors
    (`self.K2_DestroyActor` _array_element))
  (`self.InitLevel` :!label _label)
  (bind _returnvalue (`|CreateWidget` "/Game/Game/Widgets/WBP_UpgradeWidget.WBP_UpgradeWidget_C" (`GameplayStatics.GetPlayerController` 0)))
  (set `/Game/Game/Widgets/WBP_UpgradeWidget.IsFirstUpgrade` true _returnvalue)
  (set `/Game/Game/Widgets/WBP_UpgradeWidget.Fightert` (`self.Player`) _returnvalue)
  (`UserWidget.AddToViewport` _returnvalue 0))

(event `self.ReceiveBeginPlay`
  (goto _label))

(event `NextFight`
  (`KismetSystemLibrary.PrintString` (`KismetStringLibrary.Concat_StrStr` "В бою: \n" (`KismetStringLibrary.Conv_IntToString` (`KismetArrayLibrary.Array_Length` (`TurnSystemManager.FightIncludedObjects` (`self.TurnSystem`)))) "пероснажа") true true (struct :`R` 0.97444 :`G` 1.0 :`B` 0.966278 :`A` 1.0) 10.0)
  (bind _newparam (`self.MobGenerator`))
  (`self.NewFight1v1` (`self.Player`) _newparam))

(event `InitPlayer`
  (bind _choosedclass (`self.ChoosedClass`))
  (set `/Game/Game/BP_PlayerFighter.ChoosedClass` _choosedclass (`self.Player`))
  (bind _returnvalue (`|GetDataTableRow` "/Game/Game/ClassBuffs/DataTables/ClassInfo/DT_Classes.DT_Classes" (`KismetStringLibrary.Conv_StringToName` (`|GetEnumeratorNameAsString` _choosedclass)))
    (:`then`
      (set `/Game/Game/BP_PlayerFighter.Class` (`|MakeMap` _choosedclass _returnvalue) (`self.Player`))
      (bind _newstats (`self.RandomizeStats`))
      (`/Game/Game/BP_Fighter.Init` (`self.Player`) _newstats)
      (bind _newparam (`self.MobGenerator`))
      (`self.NewFight1v1` (`self.Player`) _newparam))))

(event `InitLevel`
  (`/Engine/EditorBlueprintResources/StandardMacros.IsValid` (`self.TurnSystem`)
    (:`Is Valid`
      _)
    (:`Is Not Valid`
      (`KismetSystemLibrary.PrintString` "Creating TurnSystem")
      (bind _returnvalue (`|SpawnActorFromClass` "/Script/MyProject2.TurnSystemManager" (`KismetMathLibrary.MakeTransform` (0.0 0.0 0.0)) "Undefined" "MultiplyWithRoot" null null))
      (set `self.TurnSystem` _returnvalue)))
  (bind _asbp_player_controller (cast `/Game/Game/BP_PlayerController` (`GameplayStatics.GetPlayerController` 0)))
  (bind _output_get (set `self.As BP Player Controller` _asbp_player_controller))
  (bind _outactors (`GameplayStatics.GetAllActorsOfClassWithTag` "/Script/Engine.TargetPoint" "PlayerStartPos"))
  (bind _returnvalue_2 (`|SpawnActorFromClass` "/Game/Game/BP_PlayerFighter.BP_PlayerFighter_C" (`self.GetTransform` (`|GetArrayItem` _outactors)) "Undefined" "MultiplyWithRoot" null null))
  (set `/Game/Game/BP_PlayerController.MainActor` _returnvalue_2 _output_get)
  (set `self.Player` _returnvalue_2))

(event `OnEnemyDown`
  (params (DeadObject :type "TurnWorkedObject Object Reference"))
  (set `self.CountOfBeatedEnemies` (+ (`self.CountOfBeatedEnemies`) 1))
  (`TurnSystemManager.OnPlayerDeath` (`self.TurnSystem`) DeadObject)
  (`KismetSystemLibrary.PrintText` "Удален")
  (bind _returnvalue (`TurnSystemManager.GetFightIncludedObjects` (`self.TurnSystem`)))
  (bind _returnvalue_2 (`KismetArrayLibrary.Array_Length` _returnvalue))
  (if (== _returnvalue_2 1)
    (`KismetSystemLibrary.PrintString` "Бой окончен")
    (`TurnSystemManager.ClearFighters` (`self.TurnSystem`))
    (if (== (`self.CountOfBeatedEnemies`) 5)
      (`WidgetLayoutLibrary.RemoveAllWidgets`)
      (bind _returnvalue_3 (`|CreateWidget` "/Game/Game/Widgets/WBP_WinWidget1.WBP_WinWidget1_C" (`GameplayStatics.GetPlayerController` 0)))
      (`UserWidget.AddToViewport` _returnvalue_3 0)
      (`|CreateWidget` "/Game/Game/Widgets/WBP_Counter.WBP_Counter_C" (`GameplayStatics.GetPlayerController` 0)))
    (else
      (`KismetSystemLibrary.PrintString` (`KismetStringLibrary.Concat_StrStr` "Бой продолжается \n" "Колчичество челов: " (`KismetStringLibrary.Conv_IntToString` _returnvalue_2))))))

(fn `MobGenerator`
  (returns (NewParam :type "/Game/Game/BP_MobFighter Object Reference"))
  (bind _outactors (`GameplayStatics.GetAllActorsOfClassWithTag` "/Script/Engine.TargetPoint" "EnemyStartPos"))
  (bind _returnvalue (`|SpawnActorFromClass` "/Game/Game/BP_MobFighter.BP_MobFighter_C" (`self.GetTransform` (`|GetArrayItem` _outactors)) "Undefined" "MultiplyWithRoot" null null))
  (`/Game/Game/BP_Fighter.Init` _returnvalue (`|MakeMap` "NewEnumerator0" :!type "/Game/Game/Enums/E_Params Enum"))
  (return _returnvalue))

(fn `NewFight1v1`
  (params (Player :type "/Game/Game/BP_PlayerFighter Object Reference") (Mob :type "/Game/Game/BP_MobFighter Object Reference"))
  (locals (PlayerPawn :type "/Game/Game/BP_PlayerFighter Object Reference") (MobPawn :type "/Game/Game/BP_MobFighter Object Reference"))
  (`TurnSystemManager.ClearFighters` (`self.TurnSystem`))
  (set `local.PlayerPawn` Player)
  (set `local.MobPawn` Mob)
  (if (>= (`BlueprintMapLibrary.Map_Find` (`/Game/Game/BP_Fighter.Parameters` Player) "NewEnumerator1") (`BlueprintMapLibrary.Map_Find` (`/Game/Game/BP_Fighter.Parameters` Mob) "NewEnumerator1"))
    (`TurnSystemManager.AddObjectInFight` (`self.TurnSystem`) (`self.Player`))
    (`TurnSystemManager.AddObjectInFight` (`self.TurnSystem`) (`local.MobPawn`))
    (else
      (`TurnSystemManager.AddObjectInFight` (`self.TurnSystem`) (`local.MobPawn`))
      (`TurnSystemManager.AddObjectInFight` (`self.TurnSystem`) (`local.PlayerPawn`))))
  (set `/Game/Game/BP_Fighter.CurrentEnemy` (`local.MobPawn`) (`self.Player`))
  (set `/Game/Game/BP_Fighter.CurrentEnemy` (`local.PlayerPawn`) (`local.MobPawn`))
  (bind _returnvalue (`TurnSystemManager.GetFightIncludedObjects` (`self.TurnSystem`)))
  (`KismetSystemLibrary.PrintString` (`KismetStringLibrary.Conv_IntToString` (`KismetArrayLibrary.Array_Length` _returnvalue)))
  (`TurnWorkedObject.CallMakeTurn` (`|GetArrayItem` _returnvalue)))

(fn `RandomizeStats`
  (returns (NewStats :type "Map of /Game/Game/Enums/E_Params Enum to Integer"))
  (locals (Stats :type "Map of /Game/Game/Enums/E_Params Enum to Object Object Reference"))
  (`BlueprintMapLibrary.Map_Add` (`local.Stats`) "NewEnumerator0" (`KismetMathLibrary.RandomInteger` 4))
  (`BlueprintMapLibrary.Map_Add` (`local.Stats`) "NewEnumerator1" (`KismetMathLibrary.RandomInteger` 4))
  (`BlueprintMapLibrary.Map_Add` (`local.Stats`) "NewEnumerator2" (`KismetMathLibrary.RandomInteger` 4))
  (return (`local.Stats`)))

(fn `UserConstructionScript`)