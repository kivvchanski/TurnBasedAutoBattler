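; BP_SlashDamageResist is a class buff ability that reduces one incoming damage type, presumably slash going by the asset name.
; On Init it adds itself to the owner's DefenceAbilities array.
; CallEffect subtracts the Target's weapon damage from matching hits, clamped at zero, and passes other types through unchanged.
; It returns damage, type, target and owner, and prints debug strings along the way.
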(fn `CallEffect`
  (params (Damage :type Integer) (DamageType :type "/Game/Game/Enums/E_DamageType Enum" :default "NewEnumerator0") (Target :type "/Game/Game/BP_Fighter Object Reference") (Owner :type "/Game/Game/BP_Fighter Object Reference"))
  (returns (ODamage :type Integer) (ODamageType :type "/Game/Game/Enums/E_DamageType Enum") (OTarget :type "/Game/Game/BP_Fighter Object Reference") (OOwner :type "/Game/Game/BP_Fighter Object Reference"))
  (bind _returnvalue (`KismetMathLibrary.Max` (- Damage (`.Damage_5_B533745D4485504A44D4CCB3EE18A368` (break `/Game/Game/Weapons/ST_Weapon` (`/Game/Game/BP_Fighter.Weapon` Target))))))
  (`KismetSystemLibrary.PrintString` (`KismetStringLibrary.Concat_StrStr` "DAMAGE IN EFFECT: " (`KismetStringLibrary.Conv_IntToString` Damage)) true true (struct :`G` 0.66 :`B` 1.0 :`A` 1.0) 30.0)
  (if (`|EnumEquality` DamageType "NewEnumerator2")
    (`KismetSystemLibrary.PrintString` (`KismetStringLibrary.Concat_StrStr` "Decreasing Damage to: " (`KismetStringLibrary.Conv_IntToString` _returnvalue)))
    (return _returnvalue DamageType Target Owner)
    (else
      (return Damage DamageType Target Owner))))

(fn `Init`
  (params (Owner :type "/Game/Game/BP_Fighter Object Reference"))
  (`KismetArrayLibrary.Array_Add` (`/Game/Game/BP_Fighter.DefenceAbilities` Owner) self)
  (`parent.Init` Owner))