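; Class buff attack ability that adds turn-scaled "poison" damage to its owner's attacks.
; Init registers the ability in the owner's AtackAbilities array, then runs the parent Init.
; CallEffect adds the owner's current turn number minus one to the incoming damage, prints the total for debugging, and passes damage type, target and owner through unchanged.
; It applies no damage over time or status itself.
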(fn `CallEffect`
  (params (Damage :type Integer) (DamageType :type "/Game/Game/Enums/E_DamageType Enum" :default "NewEnumerator0") (Target :type "/Game/Game/BP_Fighter Object Reference") (Owner :type "/Game/Game/BP_Fighter Object Reference"))
  (returns (ODamage :type Integer) (ODamageType :type "/Game/Game/Enums/E_DamageType Enum") (OTarget :type "/Game/Game/BP_Fighter Object Reference") (OOwner :type "/Game/Game/BP_Fighter Object Reference"))
  (bind _returnvalue (+ Damage (- (`/Game/Game/BP_Fighter.CurrentTurnNum` Owner) 1)))
  (`KismetSystemLibrary.PrintString` (`KismetStringLibrary.Concat_StrStr` (`KismetStringLibrary.Conv_IntToString` _returnvalue) " poison damage"))
  (return _returnvalue DamageType Target Owner))

(fn `Init`
  (params (Owner :type "/Game/Game/BP_Fighter Object Reference"))
  (`KismetArrayLibrary.Array_Add` (`/Game/Game/BP_Fighter.AtackAbilities` Owner) self)
  (`parent.Init` Owner))