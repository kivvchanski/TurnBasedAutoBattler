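; BP_Shield is a class-buff defence ability that reduces incoming damage.
; Init registers it in the owner's DefenceAbilities list, then runs the parent initialisation.
; CallEffect subtracts a small flat amount from damage, clamped at zero, when the target's value for one enum-keyed parameter is lower than the owner's.
; Otherwise damage is unchanged, and damage type, target and owner always pass through.
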(fn `CallEffect`
  (params (Damage :type Integer) (DamageType :type "/Game/Game/Enums/E_DamageType Enum" :default "NewEnumerator0") (Target :type "/Game/Game/BP_Fighter Object Reference") (Owner :type "/Game/Game/BP_Fighter Object Reference"))
  (returns (ODamage :type Integer) (ODamageType :type "/Game/Game/Enums/E_DamageType Enum") (OTarget :type "/Game/Game/BP_Fighter Object Reference") (OOwner :type "/Game/Game/BP_Fighter Object Reference"))
  (if (< (`BlueprintMapLibrary.Map_Find` (`/Game/Game/BP_Fighter.Parameters` Target) "NewEnumerator0") (`BlueprintMapLibrary.Map_Find` (`/Game/Game/BP_Fighter.Parameters` Owner) "NewEnumerator0"))
    (return (`KismetMathLibrary.Max` (- Damage 3)) DamageType Target Owner)
    (else
      (return Damage DamageType Target Owner))))

(fn `Init`
  (params (Owner :type "/Game/Game/BP_Fighter Object Reference"))
  (`KismetArrayLibrary.Array_Add` (`/Game/Game/BP_Fighter.DefenceAbilities` Owner) self)
  (`parent.Init` Owner))