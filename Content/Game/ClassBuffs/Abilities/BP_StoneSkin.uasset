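; BP_StoneSkin is a class buff ability that reduces incoming damage by a flat amount.
; Init adds it to the owner's DefenceAbilities, then runs the parent Init.
; CallEffect subtracts one of the owner's Parameters values from the damage, floors the result at zero, and passes type, target and owner through unchanged.
; It also prints the unreduced damage on screen as debug output.
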(fn `CallEffect`
  (params (Damage :type Integer) (DamageType :type "/Game/Game/Enums/E_DamageType Enum" :default "NewEnumerator0") (Target :type "/Game/Game/BP_Fighter Object Reference") (Owner :type "/Game/Game/BP_Fighter Object Reference"))
  (returns (ODamage :type Integer) (ODamageType :type "/Game/Game/Enums/E_DamageType Enum") (OTarget :type "/Game/Game/BP_Fighter Object Reference") (OOwner :type "/Game/Game/BP_Fighter Object Reference"))
  (bind _returnvalue (- Damage (`BlueprintMapLibrary.Map_Find` (`/Game/Game/BP_Fighter.Parameters` Owner) "NewEnumerator2")))
  (`KismetSystemLibrary.PrintString` (`KismetStringLibrary.Concat_StrStr` "DAMAGE IN EFFECT: " (`KismetStringLibrary.Conv_IntToString` Damage)) true true (struct :`G` 0.66 :`B` 1.0 :`A` 1.0) 30.0)
  (if (> _returnvalue 0)
    (return _returnvalue DamageType Target Owner)
    (else
      (return 0 DamageType Target Owner))))

(fn `Init`
  (params (Owner :type "/Game/Game/BP_Fighter Object Reference"))
  (`KismetArrayLibrary.Array_Add` (`/Game/Game/BP_Fighter.DefenceAbilities` Owner) self)
  (`parent.Init` Owner))