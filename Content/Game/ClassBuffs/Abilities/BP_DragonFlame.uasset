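; BP_DragonFlame is a class-buff attack ability that periodically boosts its owner's damage with a flame burst.
; Init registers it in the owner's attack abilities list.
; CallEffect adds a flat damage bonus whenever the owner's turn number is divisible by three, calling EmitFlame if that owner is a BP_MobFighter.
; Damage type, target and owner pass through unchanged, as does damage on other turns.
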(fn `CallEffect`
  (params (Damage :type Integer) (DamageType :type "/Game/Game/Enums/E_DamageType Enum" :default "NewEnumerator0") (Target :type "/Game/Game/BP_Fighter Object Reference") (Owner :type "/Game/Game/BP_Fighter Object Reference"))
  (returns (ODamage :type Integer) (ODamageType :type "/Game/Game/Enums/E_DamageType Enum") (OTarget :type "/Game/Game/BP_Fighter Object Reference") (OOwner :type "/Game/Game/BP_Fighter Object Reference"))
  (if (== (mod (`/Game/Game/BP_Fighter.CurrentTurnNum` Owner) 3) 0)
    (bind _asbp_mob_fighter (cast `/Game/Game/BP_MobFighter` Owner)
      (:`then`
        (`/Game/Game/BP_MobFighter.EmitFlame` _asbp_mob_fighter))
      (:`CastFailed`
        _))
    (return (+ Damage 3) DamageType Target Owner)
    (else
      (return Damage DamageType Target Owner))))

(fn `Init`
  (params (Owner :type "/Game/Game/BP_Fighter Object Reference"))
  (`KismetArrayLibrary.Array_Add` (`/Game/Game/BP_Fighter.AtackAbilities` Owner) self))