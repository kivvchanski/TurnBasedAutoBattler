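; Class buff ability for a sneak attack that gives its owner a conditional damage bonus.
; Init registers the ability in the owner's AtackAbilities, then calls the parent Init.
; CallEffect adds one damage when the owner's value for one enum-keyed parameter strictly exceeds the target's, passing damage type, target and owner through unchanged.
; Both functions print debug strings.
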(fn `CallEffect`
  (params (Damage :type Integer) (DamageType :type "/Game/Game/Enums/E_DamageType Enum" :default "NewEnumerator0") (Target :type "/Game/Game/BP_Fighter Object Reference") (Owner :type "/Game/Game/BP_Fighter Object Reference"))
  (returns (ODamage :type Integer) (ODamageType :type "/Game/Game/Enums/E_DamageType Enum") (OTarget :type "/Game/Game/BP_Fighter Object Reference") (OOwner :type "/Game/Game/BP_Fighter Object Reference"))
  (`KismetSystemLibrary.PrintString` "So sneaky")
  (if (> (`BlueprintMapLibrary.Map_Find` (`/Game/Game/BP_Fighter.Parameters` Owner) "NewEnumerator1") (`BlueprintMapLibrary.Map_Find` (`/Game/Game/BP_Fighter.Parameters` Target) "NewEnumerator1"))
    (return (+ Damage 1) DamageType Target Owner)
    (else
      (return Damage DamageType Target Owner))))

(fn `Init`
  (params (Owner :type "/Game/Game/BP_Fighter Object Reference"))
  (`KismetSystemLibrary.PrintString` "+ sneaky atack")
  (`KismetArrayLibrary.Array_Add` (`/Game/Game/BP_Fighter.AtackAbilities` Owner) self)
  (`parent.Init` Owner))