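; BP_RushAction is a class buff attack ability that boosts a fighter's damage during its first turn.
; Init registers the ability in the owner's attack ability list.
; CallEffect adds the owner's weapon damage when CurrentTurnNum is 1, passing damage type, target and owner through unchanged.
; BeginPlay binds UpdateState to the owning BP_Fighter's update event, but that handler is empty.
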(event `self.ReceiveBeginPlay`
  (bind _asbp_fighter (cast `/Game/Game/BP_Fighter` (`self.GetOwner`)))
  (add `/Game/Game/BP_Fighter.Update` _asbp_fighter (delegate `UpdateState`)))

(event `UpdateState`)

(fn `CallEffect`
  (params (Damage :type Integer) (DamageType :type "/Game/Game/Enums/E_DamageType Enum" :default "NewEnumerator0") (Target :type "/Game/Game/BP_Fighter Object Reference") (Owner :type "/Game/Game/BP_Fighter Object Reference"))
  (returns (ODamage :type Integer) (ODamageType :type "/Game/Game/Enums/E_DamageType Enum") (OTarget :type "/Game/Game/BP_Fighter Object Reference") (OOwner :type "/Game/Game/BP_Fighter Object Reference"))
  (if (== (`/Game/Game/BP_Fighter.CurrentTurnNum` Owner) 1)
    (`KismetSystemLibrary.PrintString` "Rush action activated")
    (return (+ Damage (`.Damage_5_B533745D4485504A44D4CCB3EE18A368` (break `/Game/Game/Weapons/ST_Weapon` (`/Game/Game/BP_Fighter.Weapon` Owner)))) DamageType Target Owner)
    (else
      (return Damage DamageType Target Owner))))

(fn `Init`
  (params (Owner :type "/Game/Game/BP_Fighter Object Reference"))
  (bind _atackabilities (`/Game/Game/BP_Fighter.AtackAbilities` Owner))
  (`KismetArrayLibrary.Array_Add` _atackabilities self)
  (set `/Game/Game/BP_Fighter.AtackAbilities` _atackabilities Owner)
  (`parent.Init` Owner))

(fn `Refresh`
  (`parent.Refresh`))