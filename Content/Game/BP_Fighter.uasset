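; BP_Fighter is a base turn-based combat fighter with random starting stats, HP and an HP widget link.
; Each turn rolls a dexterity-based hit check against the current enemy, then adds a stat bonus to weapon damage.
; Attack and defence ability lists act as perk chains, each effect passing damage, type and target to the next.
; Incoming damage reduces HP, and death notifies the game state.
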(event `self.ReceiveBeginPlay`
  (bind _enumvalue (foreach `/Game/Game/Enums/E_Params` false)
    (:`LoopBody`
      (`BlueprintMapLibrary.Map_Add` (`self.Parameters`) _enumvalue (`KismetMathLibrary.RandomIntegerInRange` 1 3)))))

(event `self.MakeTurn`
  (set `self.CurrentTurnNum` (+ (`self.CurrentTurnNum`) 1))
  (`self.AtackEvent`)
  (`KismetSystemLibrary.Delay` 2.0))

(event `AtackEvent`
  (bind (_name _damage _model _damagetype) (break `/Game/Game/Weapons/ST_Weapon` (`self.Weapon`)))
  (bind _hit (`self.TryHit`))
  (if _hit
    (`self.HitedAtack`)
    (bind _output_get (set `self.CurrentDamage` (+ _damage (`BlueprintMapLibrary.Map_Find` (`self.Parameters`) "NewEnumerator0"))))
    (bind (_odamage _otype) (`self.UseAllPerks` (`self.AtackAbilities`) _output_get _damagetype (`self.CurrentEnemy`)))
    (`KismetSystemLibrary.PrintString` (`KismetStringLibrary.Concat_StrStr` "OUTPUT DAMAGE: " (`KismetStringLibrary.Conv_IntToString` _odamage)) true true (struct :`G` 0.66 :`B` 1.0 :`A` 1.0) 30.0)
    (`self.TakeDamage` (`self.CurrentEnemy`) _odamage _otype self)
    (else
      (`self.NotHitedAtack`))))

(event `TakeDamage`
  (params (Damage :type Integer) (AtackType :type "/Game/Game/Enums/E_DamageType Enum" :default "NewEnumerator0") (AtackingFighterRef :type "/Game/Game/BP_Fighter Object Reference"))
  (`KismetSystemLibrary.PrintString` (`KismetStringLibrary.Concat_StrStr` "INPUT DAMAGE: " (`KismetStringLibrary.Conv_IntToString` Damage)) true true (struct :`G` 0.66 :`B` 1.0 :`A` 1.0) 30.0)
  (bind _odamage (`self.UseAllPerks` (`self.DefenceAbilities`) Damage AtackType AtackingFighterRef))
  (set `self.HP` (- (`self.HP`) _odamage))
  (`KismetSystemLibrary.PrintString` (`KismetStringLibrary.Concat_StrStr` "I get " (`KismetStringLibrary.Conv_IntToString` _odamage) " damage") true true (struct :`R` 0.011738 :`G` 1.0 :`A` 1.0) 30.0)
  (if (<= (`self.HP`) 0)
    (`self.Death`)))

(event `RefreshAll`
  (`self.RefreshAbilities`)
  (`self.RefreshChar`)
  (set `self.CurrentTurnNum` 0))

(event `Death`
  (`KismetSystemLibrary.PrintString` "I'm dying")
  (bind _asbp_game_state (cast `/Game/Game/BP_GameState` (`GameplayStatics.GetGameState`)))
  (`/Game/Game/BP_GameState.OnEnemyDown` _asbp_game_state self))

(event `HitedAtack`)

(event `NotHitedAtack`)

(fn `AddStat`
  (params (Param :type "/Game/Game/Enums/E_Params Enum" :default "NewEnumerator0") (Count :type Integer))
  (`BlueprintMapLibrary.Map_Add` (`self.Parameters`) Param (+ (`BlueprintMapLibrary.Map_Find` (`self.Parameters`) Param) Count)))

(fn `Init`
  (params (Stats :type "Map of /Game/Game/Enums/E_Params Enum to Integer"))
  (set `self.Parameters` Stats)
  (bind _aswbp_hpwidget (cast `/Game/Game/Widgets/WBP_HPWidget` (`WidgetComponent.GetWidget` (`self.Widget`))))
  (set `/Game/Game/Widgets/WBP_HPWidget.TargetFighter` self _aswbp_hpwidget))

(fn `MakeTurn2`)

(fn `RefreshAbilities`
  (for _array_element (`self.AtackAbilities`)
    (`/Game/Game/ClassBuffs/Abilities/BP_BaseAbility.Refresh` _array_element)
    (for _array_element_2 (`self.DefenceAbilities`)
      (`/Game/Game/ClassBuffs/Abilities/BP_BaseAbility.Refresh` _array_element_2))))

(fn `RefreshChar`
  (set `self.HP` (`self.MaxHP`))
  (set `self.CurrentTurnNum` 0))

(fn `TryHit`
  (returns (Hit :type Boolean))
  (locals (HitResult :type Integer))
  (bind _currentenemy (`self.CurrentEnemy`))
  (bind _value (`BlueprintMapLibrary.Map_Find` (`/Game/Game/BP_Fighter.Parameters` _currentenemy) "NewEnumerator1"))
  (bind _returnvalue (+ (`BlueprintMapLibrary.Map_Find` (`self.Parameters`) "NewEnumerator1") _value))
  (`/Engine/EditorBlueprintResources/StandardMacros.IsValid` _currentenemy
    (:`Is Valid`
      (bind _output_get (set `local.HitResult` (`KismetMathLibrary.RandomIntegerInRange` 1 _returnvalue)))
      (bind _returnvalue_2 (> _output_get _value))
      (`KismetSystemLibrary.PrintString` (`KismetStringLibrary.Concat_StrStr` "I'm trying to hit... \n" "Sum of our dex is " (`KismetStringLibrary.Conv_IntToString` _returnvalue) " \nMy result is " (`KismetStringLibrary.Conv_IntToString` _output_get) " \nDex of my oponent: " (`KismetStringLibrary.Conv_IntToString` _value) " \nresult in func: " (`KismetStringLibrary.Conv_BoolToString` _returnvalue_2)) true true (struct :`R` 0.880208 :`G` 0.121814 :`A` 1.0) 10.0)
      (return _returnvalue_2))))

(fn `UseAllPerks`
  (params (Abilities :type "Array of /Game/Game/ClassBuffs/Abilities/BP_BaseAbility Object Reference") (Damage :type Integer) (Type :type "/Game/Game/Enums/E_DamageType Enum" :default "NewEnumerator0") (Enemy :type "/Game/Game/BP_Fighter Object Reference"))
  (returns (ODamage :type Integer) (OType :type "/Game/Game/Enums/E_DamageType Enum") (OEnemy :type "/Game/Game/BP_Fighter Object Reference"))
  (locals (CurDamage :type Integer) (CurType :type "/Game/Game/Enums/E_DamageType Enum" :default "NewEnumerator0") (CurEnemy :type "/Game/Game/BP_Fighter Object Reference"))
  (bind _output_get (set `local.CurDamage` Damage))
  (`KismetSystemLibrary.PrintString` "SET DAMAGE AT: " true true (struct :`G` 0.66 :`B` 1.0 :`A` 1.0) 30.0)
  (`KismetSystemLibrary.PrintString` (`KismetStringLibrary.Conv_IntToString` _output_get) true true (struct :`G` 0.66 :`B` 1.0 :`A` 1.0) 30.0)
  (set `local.CurType` Type)
  (set `local.CurEnemy` Enemy)
  (for _array_element Abilities
    (bind (_odamage _odamagetype _otarget) (`/Game/Game/ClassBuffs/Abilities/BP_BaseAbility.CallEffect` _array_element (`local.CurDamage`) (`local.CurType`) (`local.CurEnemy`) self))
    (set `local.CurDamage` _odamage)
    (set `local.CurType` _odamagetype)
    (set `local.CurEnemy` _otarget)
    (`KismetSystemLibrary.PrintString` (`KismetStringLibrary.Concat_StrStr` "Call effect: " (`KismetSystemLibrary.GetObjectName` _array_element) " \nDamage: \n" (`KismetStringLibrary.Conv_IntToString` _odamage)) true true (struct :`R` 0.54993 :`G` 0.192543 :`B` 1.0 :`A` 1.0) 30.0))
  (return (`local.CurDamage`) (`local.CurType`) (`local.CurEnemy`)))

(fn `UserConstructionScript`)