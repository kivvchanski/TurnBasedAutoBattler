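; Player controller that drives the HUD and the reward flow between fights for its MainActor fighter.
; It adds a counter widget on start and shows a parameters view while C is held.
; GetPrize refreshes the fighter and shows a new-weapon widget from the DT_Weapons row at that index.
; Widget events chain weapon selection into the upgrade screen, whose completion calls NextFight on BP_GameState.
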(event `self.ReceiveBeginPlay`
  (bind _returnvalue (`|CreateWidget` "/Game/Game/Widgets/WBP_Counter.WBP_Counter_C" self))
  (`UserWidget.AddToViewport` _returnvalue 0))

(event `Key|LeftMouseButton`
  (params (Key :type "Key Structure")))

(event `GetPrize`
  (params (WeaponID :type Integer))
  (`/Game/Game/BP_Fighter.RefreshAll` (`self.MainActor`))
  (bind _outrownames (`DataTableFunctionLibrary.GetDataTableRowNames` "/Game/Game/Weapons/DT_Weapons.DT_Weapons"))
  (bind _returnvalue (`|GetDataTableRow` "/Game/Game/Weapons/DT_Weapons.DT_Weapons" (`|GetArrayItem` _outrownames WeaponID))
    (:`then`
      (bind _returnvalue_2 (`|CreateWidget` "/Game/Game/Widgets/WBP_GetNewWeapob.WBP_GetNewWeapob_C" self))
      (set `/Game/Game/Widgets/WBP_GetNewWeapob.Weapon` _returnvalue _returnvalue_2)
      (add `/Game/Game/Widgets/WBP_GetNewWeapob.WeaponSelected` _returnvalue_2 (delegate `Upgrade`))
      (`KismetSystemLibrary.PrintString` "Забижено")
      (`UserWidget.AddToViewport` _returnvalue_2 0))))

(event `Upgrade`
  (bind _returnvalue (`|CreateWidget` "/Game/Game/Widgets/WBP_UpgradeWidget.WBP_UpgradeWidget_C" self))
  (set `/Game/Game/Widgets/WBP_UpgradeWidget.Fightert` (`self.MainActor`) _returnvalue)
  (add `/Game/Game/Widgets/WBP_UpgradeWidget.Upgraded` _returnvalue (delegate `Start next fight`))
  (`UserWidget.AddToViewport` _returnvalue 0))

(event `Key|C`
  (params (Key :type "Key Structure"))
  (:`Pressed`
    (bind _returnvalue (`|CreateWidget` "/Game/Game/Widgets/WBP_ParametersView.WBP_ParametersView_C" self))
    (set `/Game/Game/Widgets/WBP_ParametersView.Fighter` (`self.MainActor`) _returnvalue)
    (`UserWidget.AddToViewport` _returnvalue 0))
  (:`Released`
    (`Widget.RemoveFromParent` _returnvalue)))

(event `Start next fight`
  (bind _asbp_game_state (cast `/Game/Game/BP_GameState` (`GameplayStatics.GetGameState`)))
  (`/Game/Game/BP_GameState.NextFight` _asbp_game_state))

(fn `UserConstructionScript`)