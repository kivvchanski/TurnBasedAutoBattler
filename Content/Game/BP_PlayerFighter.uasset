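; Player fighter for turn-based combat: it registers with the player camera and HP widget, and shows a lose screen on death.
; Init loads the chosen class, weapon and first ability from data tables and randomizes stats.
; LevelUp supports multiclassing through a class map, adding per-level skill components and stat bonuses, then recalculating and refilling HP.
; Each turn plays an attack montage, whose notify drives the parent attack and whose completion passes the turn.
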(event `self.ReceiveBeginPlay`
  (`KismetSystemLibrary.Delay` 0.2)
  (bind _asbp_player_camera (cast `/Game/Game/BP_PlayerCamera` (`GameplayStatics.GetPlayerPawn` 0)))
  (set `/Game/Game/BP_PlayerCamera.MainActor` self _asbp_player_camera)
  (bind _aswbp_hpwidget (cast `/Game/Game/Widgets/WBP_HPWidget` (`WidgetComponent.GetWidget` (`self.Widget`))))
  (set `/Game/Game/Widgets/WBP_HPWidget.TargetFighter` self _aswbp_hpwidget)
  (`parent.ReceiveBeginPlay`))

(event `self.TakeDamage`
  (params (Damage :type Integer) (AtackType :type "/Game/Game/Enums/E_DamageType Enum" :default "NewEnumerator0") (AtackingFighterRef :type "/Game/Game/BP_Fighter Object Reference"))
  (`parent.TakeDamage` Damage AtackType AtackingFighterRef)
  (`KismetSystemLibrary.PrintString` "Я могу чувствовать боль"))

(event `self.MakeTurn`
  (`/Engine/EditorBlueprintResources/StandardMacros.IncrementInt` (`self.CurrentTurnNum`)
    (:`  `
      (`KismetSystemLibrary.PrintString` (`KismetStringLibrary.Concat_StrStr` "It's a  PlayerPawn turn") true true (struct :`G` 0.66 :`B` 1.0 :`A` 1.0) 10.0)
      (`self.AtackEvent`))))

(event `self.Death`
  (cast `/Game/Game/BP_GameState` (`GameplayStatics.GetGameState`))
  (bind _returnvalue (`|CreateWidget` "/Game/Game/Widgets/WBP_LoseWidget.WBP_LoseWidget_C" (`GameplayStatics.GetPlayerController` 0)))
  (`UserWidget.AddToViewport` _returnvalue 0)
  (`self.K2_DestroyActor`))

(event `self.AtackEvent`
  (bind _notifyname (`|PlayMontage` (`self.SkeletalMesh`) "/Game/Game/Models/Anims/AM_PaladinAtack.AM_PaladinAtack")
    (:`OnCompleted`
      (`self.PassTurn`)
      (`KismetSystemLibrary.PrintString` "PLAYER passed"))
    (:`OnNotifyBegin`
      (if (== _notifyname "Atack")
        (`parent.AtackEvent`)))))

(fn `Init`
  (params (Stats :type "Map of /Game/Game/Enums/E_Params Enum to Integer" :default _))
  (locals (ClassInfo :type "/Game/Game/ClassBuffs/DataTables/ClassInfo/ST_ClassInfo Structure") (SumMaxHp :type Integer))
  (bind _class (`self.Class`))
  (bind (_currentlevel _abilities _hpperlvl _startweaponid) (break `/Game/Game/ClassBuffs/DataTables/ClassInfo/ST_ClassInfo` (`local.ClassInfo`)))
  (set `self.Parameters` Stats)
  (set `self.CurrentLevel` 1)
  (switch `/Game/Game/Enums/E_Classes` (`self.ChoosedClass`)
    (:`NewEnumerator0`
      (bind _returnvalue (`|GetDataTableRow` "/Game/Game/ClassBuffs/DataTables/ClassInfo/DT_Classes.DT_Classes" "Warrior")
        (:`then`
          (`KismetSystemLibrary.PrintString` "Yourchoice is a Warior")
          (set `local.ClassInfo` _returnvalue))))
    (:`NewEnumerator1`
      (bind _returnvalue_2 (`|GetDataTableRow` "/Game/Game/ClassBuffs/DataTables/ClassInfo/DT_Classes.DT_Classes" "Barbarian")
        (:`then`
          (`KismetSystemLibrary.PrintString` "Yourchoice is a Barbarian")
          (set `local.ClassInfo` _returnvalue_2))))
    (:`NewEnumerator2`
      (bind _returnvalue_3 (`|GetDataTableRow` "/Game/Game/ClassBuffs/DataTables/ClassInfo/DT_Classes.DT_Classes" "Rogue")
        (:`then`
          (`KismetSystemLibrary.PrintString` "Yourchoice is a rogue")
          (set `local.ClassInfo` _returnvalue_3)))))
  (set `self.HpPerLevel` _hpperlvl)
  (set `self.BuffsTable` _abilities)
  (bind _returnvalue_4 (`|GetDataTableRow` "/Game/Game/Weapons/DT_Weapons.DT_Weapons" _startweaponid)
    (:`then`
      (set `self.Weapon` _returnvalue_4)
      (bind _returnvalue_5 (`|GetDataTableRow` (`self.BuffsTable`) "1")
        (:`then`
          (bind (_level _slkill _bonusstats _statcount) (break `/Game/Game/ClassBuffs/DataTables/ClassInfo/ST_BuffPerLevel` _returnvalue_5))
          (if (`KismetSystemLibrary.IsValidClass` _slkill)
            (bind _returnvalue_6 (`|AddComponentByClass` _slkill))
            (`/Game/Game/ClassBuffs/Abilities/BP_BaseAbility.Init` _returnvalue_6 self))
          (`self.AddStat` _bonusstats _statcount)
          (bind _enumvalue (foreach `/Game/Game/Enums/E_Params` false)
            (:`LoopBody`
              (`BlueprintMapLibrary.Map_Add` (`self.Parameters`) _enumvalue (`KismetMathLibrary.RandomIntegerInRange` 1 3))
              (bind _keys (`BlueprintMapLibrary.Map_Keys` _class))
              (for _array_element _keys
                (bind (_value _returnvalue_7) (`BlueprintMapLibrary.Map_Find` _class _array_element))
                (if _returnvalue_7
                  (bind (_currentlevel_2 _abilities_2 _hpperlvl_2) (break `/Game/Game/ClassBuffs/DataTables/ClassInfo/ST_ClassInfo` _value))
                  (set `local.SumMaxHp` (+ (`local.SumMaxHp`) (* _hpperlvl_2 _currentlevel_2)))))
              (bind _output_get (set `self.MaxHP` (+ (`local.SumMaxHp`) (`BlueprintMapLibrary.Map_Find` (`self.Parameters`) "NewEnumerator2"))))
              (bind _output_get_2 (set `self.HP` _output_get))
              (`KismetSystemLibrary.PrintString` "My HP is ")
              (`KismetSystemLibrary.PrintString` (`KismetStringLibrary.Conv_IntToString` _output_get_2)))))))))

(fn `LevelUp`
  (params (NewClass :type "/Game/Game/Enums/E_Classes Enum" :default "NewEnumerator0"))
  (locals (UpgradedClass :type "/Game/Game/Enums/E_Classes Enum" :default "NewEnumerator0") (NewHp :type Integer) (TotalLVL :type Integer))
  (bind _parameters (`self.Parameters`))
  (bind _class (`self.Class`))
  (bind _value (`BlueprintMapLibrary.Map_Find` (`self.Class`) (`local.UpgradedClass`)))
  (bind (_currentlevel _abilities _hpperlvl _startweaponid) (break `/Game/Game/ClassBuffs/DataTables/ClassInfo/ST_ClassInfo` (`BlueprintMapLibrary.Map_Find` (`self.Class`) (`local.UpgradedClass`))))
  (set `local.UpgradedClass` NewClass)
  (if (`.ReturnValue` (`BlueprintMapLibrary.Map_Find` (`self.Class`) NewClass))
    (`BlueprintMapLibrary.Map_Add` (`self.Class`) (`local.UpgradedClass`) (make `/Game/Game/ClassBuffs/DataTables/ClassInfo/ST_ClassInfo` (+ _currentlevel 1) _abilities _hpperlvl _startweaponid))
    (bind _returnvalue (`|GetDataTableRow` (`.Abilities_8_02DCA86943357B24C6479CB83701FDCE` (break `/Game/Game/ClassBuffs/DataTables/ClassInfo/ST_ClassInfo` _value)) (`KismetStringLibrary.Conv_StringToName` (`KismetStringLibrary.Conv_IntToString` (break `/Game/Game/ClassBuffs/DataTables/ClassInfo/ST_ClassInfo` _value))) :!label _label)
      (:`then`
        (bind (_level _slkill _bonusstats _statcount) (break `/Game/Game/ClassBuffs/DataTables/ClassInfo/ST_BuffPerLevel` _returnvalue))
        (if (`KismetSystemLibrary.IsValidClass` _slkill)
          (bind _returnvalue_2 (`|AddComponentByClass` _slkill))
          (`/Game/Game/ClassBuffs/Abilities/BP_BaseAbility.Init` _returnvalue_2 self))
        (`BlueprintMapLibrary.Map_Add` _parameters _bonusstats (+ (`BlueprintMapLibrary.Map_Find` _parameters _bonusstats) _statcount))
        (bind _keys (`BlueprintMapLibrary.Map_Keys` _class))
        (for _array_element _keys
          (bind _value_2 (`BlueprintMapLibrary.Map_Find` _class _array_element))
          (set `local.NewHp` (+ (`local.NewHp`) (* (`.HPPerLVL_11_7A2F9BFB440719ECD15EF18478AE657A` (break `/Game/Game/ClassBuffs/DataTables/ClassInfo/ST_ClassInfo` _value_2)) (break `/Game/Game/ClassBuffs/DataTables/ClassInfo/ST_ClassInfo` _value_2))))
          (set `local.TotalLVL` (+ (`local.TotalLVL`) (break `/Game/Game/ClassBuffs/DataTables/ClassInfo/ST_ClassInfo` _value_2))))
        (bind _output_get (set `local.NewHp` (+ (`local.NewHp`) (* (`BlueprintMapLibrary.Map_Find` (`self.Parameters`) "NewEnumerator2") (`local.TotalLVL`)))))
        (bind _output_get_2 (set `self.MaxHP` _output_get))
        (set `self.HP` _output_get_2)))
    (else
      (bind _returnvalue_3 (`|GetDataTableRow` "/Game/Game/ClassBuffs/DataTables/ClassInfo/DT_Classes.DT_Classes" (`KismetStringLibrary.Conv_StringToName` (`|GetEnumeratorNameAsString` (`local.UpgradedClass`))))
        (:`then`
          (`BlueprintMapLibrary.Map_Add` (`self.Class`) (`local.UpgradedClass`) _returnvalue_3)
          (goto _label))
        (:`RowNotFound`
          (`KismetSystemLibrary.PrintString` "I lost class :("))))))

(fn `MakeTurn2`)

(fn `NewFunction_0`)

(fn `UserConstructionScript`
  (`parent.UserConstructionScript`))