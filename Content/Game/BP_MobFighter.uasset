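; BP_MobFighter is an enemy fighter in turn-based combat, built on a parent fighter class.
; Init links the HP widget and picks a random DT_Mobs row for mesh, animation, stats, weapon, prize and dynamically added ability components.
; Each turn plays the attack montage, triggers the parent attack on its notify, then passes on completion.
; Death awards the prize through BP_PlayerController, then destroys the actor.
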(event `self.ReceiveBeginPlay`
  (if (`self.NewVar`)
    (`self.Init` (`|MakeMap` "NewEnumerator0" :!type "/Game/Game/Enums/E_Params Enum"))))

(event `EmitFlame`
  (`AddComponent|NODE_AddNiagaraComponent-1` :`RelativeTransform` (`SceneComponent.GetSocketTransform` (`self.SkeletalMesh`) "Tongue01Socket" "RTS_Actor"))
  (`KismetSystemLibrary.PrintString` "Flame emited"))

(event `self.Death`
  (bind _asbp_player_controller (cast `/Game/Game/BP_PlayerController` (`GameplayStatics.GetPlayerController` 0)))
  (`/Game/Game/BP_PlayerController.GetPrize` _asbp_player_controller (- (`self.PrizeItemID`) 1))
  (`parent.Death`)
  (`self.K2_DestroyActor`))

(event `self.MakeTurn`
  (`/Engine/EditorBlueprintResources/StandardMacros.IncrementInt` (`self.CurrentTurnNum`)
    (:`  `
      (`self.AtackEvent`))))

(event `self.AtackEvent`
  (bind _atackmontage (`self.AtackMontage`))
  (`/Engine/EditorBlueprintResources/StandardMacros.IsValid` _atackmontage
    (:`Is Valid`
      (bind _notifyname (`|PlayMontage` (`self.SkeletalMesh`) _atackmontage)
        (:`OnCompleted`
          (`self.PassTurn`)
          (`KismetSystemLibrary.PrintString` "MOB passed"))
        (:`OnNotifyBegin`
          (if (== _notifyname "Atack")
            (`parent.AtackEvent`)))))))

(event `self.TakeDamage`
  (params (Damage :type Integer) (AtackType :type "/Game/Game/Enums/E_DamageType Enum" :default "NewEnumerator0") (AtackingFighterRef :type "/Game/Game/BP_Fighter Object Reference"))
  (`parent.TakeDamage` Damage AtackType AtackingFighterRef))

(fn `Init`
  (params (Stats :type "Map of /Game/Game/Enums/E_Params Enum to Integer" :default _))
  (locals (NewLocalVar :type Name))
  (bind _aswbp_hpwidget (cast `/Game/Game/Widgets/WBP_HPWidget` (`WidgetComponent.GetWidget` (`self.Widget`))))
  (set `/Game/Game/Widgets/WBP_HPWidget.TargetFighter` self _aswbp_hpwidget)
  (bind _outrownames (`DataTableFunctionLibrary.GetDataTableRowNames` "/Game/Game/ClassBuffs/DataTables/DT_Mobs.DT_Mobs"))
  (set `local.NewLocalVar` (`KismetArrayLibrary.Array_Random` _outrownames))
  (`KismetSystemLibrary.PrintString` (`KismetStringLibrary.Conv_NameToString` (`local.NewLocalVar`)) true true (struct :`G` 1.0 :`B` 0.040223 :`A` 1.0) 10.0)
  (bind _returnvalue (`|GetDataTableRow` "/Game/Game/ClassBuffs/DataTables/DT_Mobs.DT_Mobs" (`local.NewLocalVar`))
    (:`then`
      (bind (_name _params _maxhp _weapondamage _abilities _priceweaponid _mesh _animbpref _atackmontage) (break `/Game/Game/ClassBuffs/DataTables/ST_MobInfo` _returnvalue))
      (set `self.Parameters` _params)
      (set `self.AtackMontage` _atackmontage)
      (set `self.PrizeItemID` _priceweaponid)
      (`SkeletalMeshComponent.SetSkeletalMeshAsset` (`self.SkeletalMesh`) _mesh)
      (bind _output_get (set `self.MaxHP` _maxhp))
      (set `self.HP` _output_get)
      (set `self.Weapon` (make `/Game/Game/Weapons/ST_Weapon` "MobWeapon" _weapondamage null))
      (`SkeletalMeshComponent.SetAnimInstanceClass` (`self.SkeletalMesh`) _animbpref)
      (`KismetSystemLibrary.PrintString` (`KismetStringLibrary.Concat_StrStr` "ТВОЙ ПРОТИВНИК: \n \n" _name) true true (struct :`R` 1.0 :`G` 0.063982 :`B` 0.068756 :`A` 1.0) 30.0)
      (for _array_element _abilities
        (bind _returnvalue_2 (`|AddComponentByClass` _array_element))
        (`/Game/Game/ClassBuffs/Abilities/BP_BaseAbility.Init` _returnvalue_2 self)))))

(fn `UserConstructionScript`
  (`parent.UserConstructionScript`))